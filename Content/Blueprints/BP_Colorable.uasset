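; BP_Colorable is an actor with a configurable static mesh whose material can be tinted.
; The construction script assigns Mesh to ColorableMesh, creates a dynamic material instance on the first material slot and sets its Color parameter to the first entry in Colors.
; BeginPlay creates the dynamic material instance again and stores it in DynaMat, without setting a color.
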(event `self.ReceiveBeginPlay`
  (bind _returnvalue (`PrimitiveComponent.CreateDynamicMaterialInstance` (`self.ColorableMesh`) 0 null))
  (set `self.DynaMat` _returnvalue))

(fn `UserConstructionScript`
  (`StaticMeshComponent.SetStaticMesh` (`self.ColorableMesh`) (`self.Mesh`))
  (bind _returnvalue (`PrimitiveComponent.CreateDynamicMaterialInstance` (`self.ColorableMesh`) 0 null))
  (set `self.DynaMat` _returnvalue)
  (`MaterialInstanceDynamic.SetVectorParameterValue` (`self.DynaMat`) "Color" (`|GetArrayItem` (`self.Colors`))))