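; BP_MenuButton is a 3D color swatch button that recolors the menu's target object when interacted with.
; Shortly after BeginPlay it takes the target and its color at the button's ID from the first BP_MenuBase, then tints its cylinder through a dynamic material.
; A timeline animates the button's scale and height as it appears, and ButtonInteract copies the color to the target's dynamic material.
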(event `self.ReceiveBeginPlay`
  (bind _scene (`self.Scene`))
  (`KismetSystemLibrary.Delay` 0.02)
  (bind _returnvalue (`PrimitiveComponent.CreateDynamicMaterialInstance` (`self.Cylinder`) 0 null))
  (set `self.DynaMat` _returnvalue)
  (bind _outactors (`GameplayStatics.GetAllActorsOfClass` "/Game/Blueprints/BP_MenuBase.BP_MenuBase_C"))
  (bind _target (`/Game/Blueprints/BP_MenuBase.Target` (`|GetArrayItem` _outactors)))
  (set `self.Target` _target)
  (bind _output (`|GetArrayItem` (`/Game/Blueprints/BP_Colorable.Colors` _target) (`self.ID`)))
  (set `self.Color` _output)
  (`MaterialInstanceDynamic.SetVectorParameterValue` (`self.DynaMat`) "Color" _output)
  (bind (_direction _scale _positionz) (`Timeline|Timeline_0` :!via `PlayFromStart`)
    (:`Update`
      (`SceneComponent.SetRelativeScale3D` _scene (`KismetMathLibrary.Conv_DoubleToVector` _scale))
      (`SceneComponent.K2_SetRelativeLocation` _scene (`KismetMathLibrary.MakeVector` 0.0 0.0 (* _positionz 40.0)) false false))))

(event `ButtonInteract`
  (`MaterialInstanceDynamic.SetVectorParameterValue` (`/Game/Blueprints/BP_Colorable.DynaMat` (`self.Target`)) "Color" (`self.Color`)))

(fn `UserConstructionScript`)